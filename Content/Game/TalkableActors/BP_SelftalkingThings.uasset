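; BP_SelftalkingThings is a talkable prop, either a dead woman or dead man, whose mesh and material the construction script picks from an enum.
; Overlap by BP_Player caches the player's UI widget and shows its interaction text.
; Interaction picks a random phrase, prefixes the Name and a colon, and types it out letter by letter through the UI's reusable dynamic text widget, then returns false.
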(event EventBeginPlay)

(event Collision|EventActorBeginOverlap
  (params (OtherActor :type Actor%20Object%20Reference))
  (bind _asbp_player (Utilities|Casting|CastToBP_Player OtherActor))
  (bind _output_get (Variables|Default|SetUIWiget (Variables|/Game/Game/Actors/BP_Player.BP_Player_C|GetUI _asbp_player)))
  (Widget|SetVisibility (Variables|/Game/Game/Widgets/MainUI/WBP_UI.WBP_UI_C|GetInteractionText _output_get) "Visible"))

(event EventTick
  (params (DeltaSeconds :type Float%20%28single-precision%29)))

(fn ConstructionScript
  (bind _staticmesh (Variables|Default|GetStaticMesh))
  (bind _staticmesh_2 (Variables|Default|GetStaticMesh))
  (switch Utilities|FlowControl|Switch|SwitchonSelftalkingEnum (Variables|Default|GetEnum)
    (:NewEnumerator0
      (Components|StaticMesh|SetStaticMesh _staticmesh_2 "/Game/Game/Models/Pers/corpse/the_corpse_of_a_girl.the_corpse_of_a_girl")
      (Rendering|Material|SetMaterial _staticmesh_2 0 "/Game/Game/Models/Pers/corpse/Material_corps/the_corpse_of_a_girl_2.the_corpse_of_a_girl_2"))
    (:NewEnumerator1
      (Components|StaticMesh|SetStaticMesh _staticmesh "/Game/Game/Models/Pers/corpse/the_corpse_of_a_man.the_corpse_of_a_man")
      (Rendering|Material|SetMaterial _staticmesh 0 "/Game/Game/Models/Pers/corpse/Material_corps/the_corpse_of_a_man_2.the_corpse_of_a_man_2"))))

(fn Interaction
  (bind _uiwiget (Variables|Default|GetUIWiget))
  (bind _phrasetosay (Variables|Default|GetPhraseToSay))
  (bind _wbp_dynamictext_reusable (Variables|/Game/Game/Widgets/MainUI/WBP_UI.WBP_UI_C|GetWBP_DynamicText_reusable _uiwiget))
  (Variables|/Game/Game/Widgets/MainUI/WBP_DynamicText_reusable.WBP_DynamicText_reusable_C|SetbIsTalkingAllowed _wbp_dynamictext_reusable true)
  (Default|SayPhrase _wbp_dynamictext_reusable (Utilities|Text|ToText(String) (Utilities|String|Append (Utilities|String|Append (Variables|Default|GetName) ": ") (Utilities|String|ToString(Text) (Utilities|Array|Get(acopy) _phrasetosay (Math|Random|RandomInteger (Utilities|Array|Length _phrasetosay)))))) 0.05)
  (return false))