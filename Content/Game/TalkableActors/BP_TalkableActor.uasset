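; BP_TalkableActor is an NPC the player can talk to, configured as a Grandma or Police character.
; The construction script picks the Russian display name, skeletal mesh and material from the Actor enum.
; Overlap begin and end toggle the interaction text in the player's UI, caching that widget.
; Interaction sends a random phrase, prefixed with the name, to a dynamic text widget that types it letter by letter.
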(event EventBeginPlay)

(event Collision|EventActorBeginOverlap
  (params (OtherActor :type Actor%20Object%20Reference))
  (bind _asbp_player (Utilities|Casting|CastToBP_Player OtherActor))
  (bind _output_get (Variables|Default|SetUIWiget (Variables|/Game/Game/Actors/BP_Player.BP_Player_C|GetUI _asbp_player)))
  (Widget|SetVisibility (Variables|/Game/Game/Widgets/MainUI/WBP_UI.WBP_UI_C|GetInteractionText _output_get) "Visible"))

(event EventTick
  (params (DeltaSeconds :type Float%20%28single-precision%29)))

(event Collision|EventActorEndOverlap
  (params (OtherActor :type Actor%20Object%20Reference))
  (Utilities|Casting|CastToBP_Player OtherActor)
  (Widget|SetVisibility (Variables|/Game/Game/Widgets/MainUI/WBP_UI.WBP_UI_C|GetInteractionText (Variables|Default|GetUIWiget)) "Hidden"))

(fn ConstructionScript
  (bind _skeletalmesh (Variables|Default|GetSkeletalMesh))
  (switch Utilities|FlowControl|Switch|SwitchonEnumTalkable (Variables|Default|GetActor)
    (:NewEnumerator0
      (Variables|Default|SetName "Бабушка")
      (Components|SkeletalMesh|SetSkeletalMeshAsset _skeletalmesh "/Game/Game/Models/Pers/Grandmum/Dwarf_Idle.Dwarf_Idle")
      (Rendering|Material|SetMaterial _skeletalmesh 0 "/Game/Game/Models/Pers/Grandmum/palette_003.palette_003")
      (Transformation|SetRelativeLocation _skeletalmesh "0.000000,0.000000,-150.000000" false false))
    (:NewEnumerator1
      (Variables|Default|SetName "Полицейский")
      (Components|SkeletalMesh|SetSkeletalMeshAsset _skeletalmesh "/Game/Game/Models/Pers/Ment/Breathing_Idle__2_.Breathing_Idle__2_")
      (Rendering|Material|SetMaterial _skeletalmesh 0 "/Game/Game/Models/Pers/Ment/palette_003.palette_003")
      (Transformation|SetRelativeLocation (Variables|Default|GetSkeletalMesh) "0.000000,0.000000,-150.000000" false false))))

(fn Interaction
  (bind _uiwiget (Variables|Default|GetUIWiget))
  (bind _phrase_to_say (Variables|Default|GetPhrase%20to%20Say))
  (bind _wbp_dynamictext_reusable (Variables|/Game/Game/Widgets/MainUI/WBP_UI.WBP_UI_C|GetWBP_DynamicText_reusable _uiwiget))
  (Variables|/Game/Game/Widgets/MainUI/WBP_DynamicText_reusable.WBP_DynamicText_reusable_C|SetbIsTalkingAllowed _wbp_dynamictext_reusable true)
  (Default|SayPhrase _wbp_dynamictext_reusable (Utilities|Text|ToText(String) (Utilities|String|Append (Utilities|String|Append (Variables|Default|GetName) ": ") (Utilities|String|ToString(Text) (Utilities|Array|Get(acopy) _phrase_to_say (Math|Random|RandomInteger (Utilities|Array|Length _phrase_to_say)))))) 0.05)
  (return false))