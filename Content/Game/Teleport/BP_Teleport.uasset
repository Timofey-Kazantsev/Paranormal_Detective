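; BP_Teleport is a teleporter actor that moves an overlapping BP_Player to the linked Teleport2 actor.
; On overlap it sets the player capsule to Teleport2's root X and Y with teleport enabled, keeping the player's own Z.
; The arrival point is offset 40 units along X, with the sign chosen by comparing this actor's Box Y against Teleport2's X, a mixed-axis check.
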(event EventBeginPlay)

(event Collision|EventActorBeginOverlap
  (params (OtherActor :type Actor%20Object%20Reference))
  (bind _teleport2 (Variables|Default|GetTeleport2))
  (bind _defaultsceneroot (Variables|BP_Teleport_C|GetDefaultSceneRoot _teleport2))
  (bind _returnvalue (Transformation|GetWorldLocation _defaultsceneroot))
  (bind _asbp_player (Utilities|Casting|CastToBP_Player OtherActor))
  (if (>= (.y (Transformation|GetWorldLocation (Variables|Default|GetBox))) (.x _returnvalue))
    (Transformation|SetWorldLocation (Variables|/Game/Game/Actors/BP_Player.BP_Player_C|GetCapsule _asbp_player) (Math|Vector|MakeVector (+ (.x _returnvalue) 4e+01) (.y _returnvalue) (.z (Transformation|GetWorldLocation (Variables|/Game/Game/Actors/BP_Player.BP_Player_C|GetCapsule _asbp_player)))) false true)
    (else
      (Transformation|SetWorldLocation (Variables|/Game/Game/Actors/BP_Player.BP_Player_C|GetCapsule _asbp_player) (Math|Vector|MakeVector (+ (.x _returnvalue) -4e+01) (.y _returnvalue) (.z (Transformation|GetWorldLocation (Variables|/Game/Game/Actors/BP_Player.BP_Player_C|GetCapsule _asbp_player)))) false true))))

(event EventTick
  (params (DeltaSeconds :type Float%20%28single-precision%29)))

(fn ConstructionScript)