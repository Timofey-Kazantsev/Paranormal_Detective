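; BP_Button is an interactable button actor that toggles a linked lift between raised and lowered.
; Its Interaction function casts the Lift reference to BP_Lift, calls Up or Down based on IsUped, flips that flag and prints it for debugging.
; The event graph and construction script are empty, and a disconnected loop that would call MoveUp on every BP_Player never runs.
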(event EventBeginPlay)

(event Collision|EventActorBeginOverlap
  (params (OtherActor :type Actor%20Object%20Reference)))

(event EventTick
  (params (DeltaSeconds :type Float%20%28single-precision%29)))

(fn ConstructionScript)

(fn Interaction
  (bind _asbp_lift (Utilities|Casting|CastToBP_Lift (Variables|Default|GetLift)))
  (if (Variables|/Game/Game/Lifts/BP_Lift.BP_Lift_C|GetIsUped _asbp_lift)
    (Default|Down _asbp_lift)
    (Variables|/Game/Game/Lifts/BP_Lift.BP_Lift_C|SetIsUped _asbp_lift false)
    (else
      (Default|Up _asbp_lift)
      (Variables|/Game/Game/Lifts/BP_Lift.BP_Lift_C|SetIsUped _asbp_lift true)))
  (Development|PrintString (Utilities|String|ToString(Boolean) (Variables|/Game/Game/Lifts/BP_Lift.BP_Lift_C|GetIsUped _asbp_lift))))