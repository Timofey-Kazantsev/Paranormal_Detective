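; Player Blueprint that moves a cube and offers a Mind-powered pulse to highlight nearby active things.
; Up and Left axis inputs move the cube along world X and Y with sweep.
; Space, while Mind remains, sphere-overlaps around the cube and turns BP_ActiveThings lights green.
; After a short delay it blacks out every light in the accumulated, never-cleared list, draining Mind per entry.
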(event Input|AxisEvents|InputAxisUp
  (params (AxisValue :type Float%20%28single-precision%29))
  (bind _cube (Variables|Default|GetCube))
  (bind _returnvalue (Transformation|GetWorldLocation _cube))
  (Transformation|SetWorldLocation (Variables|Default|GetCube) (Math|Vector|MakeVector (+ (* AxisValue (Variables|Default|GetSpeed)) (.x _returnvalue)) (.y _returnvalue) (.z _returnvalue)) true false))

(event Input|AxisEvents|InputAxisLeft
  (params (AxisValue :type Float%20%28single-precision%29))
  (bind _cube (Variables|Default|GetCube))
  (bind _returnvalue (Transformation|GetWorldLocation _cube))
  (Transformation|SetWorldLocation (Variables|Default|GetCube) (Math|Vector|MakeVector (.x _returnvalue) (+ (* AxisValue (Variables|Default|GetSpeed)) (.y _returnvalue)) (.z _returnvalue)) true false))

(event Input|KeyboardEvents|SpaceBar
  (params (Key :type Key%20Structure :default "None"))
  (:Pressed
    (if (> (Variables|Default|GetMind) 0.0)
      (bind _outactors (Collision|SphereOverlapActors (Transformation|GetWorldLocation (Variables|Default|GetCube)) 3e+02 (Variables|Default|GetObject%20Types) 0 (Variables|Default|GetActors%20to%20Ignore)))
      (for _array_element _outactors
        (bind _asbp_active_things (Utilities|Casting|CastToBP_ActiveThings _array_element))
        (Utilities|Array|Add (Variables|Default|GetOut%20Actors) _asbp_active_things)
        (Rendering|Components|Light|SetLightColor (Variables|/Game/Game/Active/BP_ActiveThings.BP_ActiveThings_C|GetPointLight _asbp_active_things) "(R=0.522256,G=1.000000,B=0.203959,A=1.000000)" true)
        (Utilities|FlowControl|Delay 1.0)
        (for _array_element_2 (Variables|Default|GetOut%20Actors)
          (Rendering|Components|Light|SetLightColor (Variables|/Game/Game/Active/BP_ActiveThings.BP_ActiveThings_C|GetPointLight _array_element_2) "(R=0.000000,G=0.000000,B=0.000000,A=1.000000)" true)
          (Variables|Default|SetMind (- (Variables|Default|GetMind) 1e+01)))))))

(fn ConstructionScript)