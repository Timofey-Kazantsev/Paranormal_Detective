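; BP_Hunter is an enemy that chases BP_Player and quits the game when its Box overlaps the player.
; Each Tick it steps the Beast component by Speed toward the player on X and Y, then turns its yaw with LookAt.
; A signed X-only gap of at most 700 triggers a delayed heart sound, alongside debug prints.
; The hunter destroys itself whenever the player's Mind is non-zero.
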(event OnComponentBeginOverlap(Box)
  (params (OverlappedComponent :type Primitive%20Component%20Object%20Reference) (OtherActor :type Actor%20Object%20Reference) (OtherComp :type Primitive%20Component%20Object%20Reference) (OtherBodyIndex :type Integer) (bFromSweep :type Boolean) (SweepResult :type Hit%20Result%20Structure%20%28by%20ref%29))
  (Utilities|Casting|CastToBP_Player OtherActor)
  (Game|QuitGame 0 "Quit" false))

(event EventTick
  (params (DeltaSeconds :type Float%20%28single-precision%29))
  (bind _speed (Variables|Default|GetSpeed))
  (bind _beast (Variables|Default|Getbeast))
  (bind _beast_2 (Variables|Default|Getbeast))
  (bind _beast_3 (Variables|Default|Getbeast))
  (bind _beast_4 (Variables|Default|Getbeast))
  (bind _beast_5 (Variables|Default|Getbeast))
  (bind _beast_6 (Variables|Default|Getbeast))
  (bind _beast_7 (Variables|Default|Getbeast))
  (bind _beast_8 (Variables|Default|Getbeast))
  (bind _arrow (Variables|Default|GetArrow))
  (bind _returnvalue (Transformation|GetWorldLocation _beast_2))
  (bind _returnvalue_2 (Transformation|GetWorldLocation _beast))
  (bind _returnvalue_3 (Transformation|GetWorldLocation _beast_5))
  (bind _returnvalue_4 (Transformation|GetWorldLocation _beast_6))
  (bind _returnvalue_5 (Math|Vector|GetForwardVector _arrow))
  (bind _returnvalue_6 (* _speed -1.0))
  (bind _returnvalue_7 (+ (.x _returnvalue) _returnvalue_6))
  (bind _outactors (Actor|GetAllActorsOfClass "/Game/Game/Actors/BP_Player.BP_Player_C"))
  (Variables|Default|SetPlayer (Utilities|Array|Get(acopy) _outactors))
  (if (== (Variables|/Game/Game/Actors/BP_Player.BP_Player_C|GetMind (Utilities|Array|Get(acopy) _outactors)) 0.0)
    (Variables|Default|SetDirection (Transformation|GetWorldLocation (Variables|/Game/Game/Actors/BP_Player.BP_Player_C|GetCapsule (Utilities|Array|Get(acopy) _outactors))))
    (if (>= (.x (Variables|Default|GetDirection)) _returnvalue_7)
      (Transformation|SetWorldLocation _beast_4 (Math|Vector|MakeVector (+ (.x _returnvalue_2) (Variables|Default|GetSpeed)) (.y _returnvalue_2) (.z _returnvalue_2)) false false)
      (Transformation|SetWorldRotation _beast_4 "0, 0, 0" false false)
      (else
        (Transformation|SetWorldLocation _beast_3 (Math|Vector|MakeVector _returnvalue_7 (.y _returnvalue) (.z _returnvalue)) false false)
        (Transformation|SetWorldRotation _beast_3 "0, 0, 0" false false)))
    (if (>= (.y (Variables|Default|GetDirection)) (.y (Transformation|GetWorldLocation (Variables|Default|Getbeast))))
      (Transformation|SetWorldLocation _beast_8 (Math|Vector|MakeVector (.x _returnvalue_3) (+ (.y _returnvalue_3) (Variables|Default|GetSpeed)) (.z _returnvalue_3)) false false)
      (Transformation|SetWorldRotation _beast_8 "0, 0, 0" false false)
      (else
        (Transformation|SetWorldLocation _beast_7 (Math|Vector|MakeVector (.x _returnvalue_4) (+ (.y _returnvalue_4) (* (Variables|Default|GetSpeed) -1.0)) (.z _returnvalue_4)) false false)
        (Transformation|SetWorldRotation _beast_7 "0, 0, 0" false false)))
    (Transformation|SetWorldRotation (Variables|Default|Getbeast) (Math|Rotator|MakeRotator 0.0 0.0 (+ (.yaw (.rotation (Class|KismetAnimationLibrary|Lookat (Transformation|GetWorldTransform (Variables|Default|Getbeast)) (Variables|Default|GetDirection) (Math|Vector|MakeVector (* (.x _returnvalue_5) 1.0) (* (.y _returnvalue_5) 1.0) (.z _returnvalue_5)) false "0, 0, 0" 0.0))) 1.8e+02)) false false)
    (if (<= (- (.x (Variables|Default|GetDirection)) (.x (Transformation|GetWorldLocation (Variables|Default|Getbeast)))) 7e+02)
      (Development|PrintString "Hello")
      (Utilities|FlowControl|Delay 1.4)
      (Audio|PlaySound2D (Variables|Default|GetSoundHeart) 1.0 1.0 0.0 0 0)
      (else
        (Development|PrintString (Utilities|String|ToString(Float) (- (.x (Variables|Default|GetDirection)) (.x (Transformation|GetWorldLocation (Variables|Default|Getbeast))))))))
    (else
      (Actor|DestroyActor))))

(fn ConstructionScript)