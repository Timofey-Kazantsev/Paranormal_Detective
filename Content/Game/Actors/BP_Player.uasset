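; Player pawn that handles movement, footstep sounds, interface-based interaction on E, and pausing diary and menu widgets.
; Movement sweeps the capsule along the arrow's forward vector via SetWorldLocation.
; Amulet (Space) lights nearby BP_ActiveThings, while ring (C), inside SW, flip-flops SecondWorld and ThirdWorld tagged actors by hiding and shifting them vertically.
; Both abilities drain Mind, updating the HUD, and spawn a single BP_Hunter once it is empty.
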(event Custom|MoveUp
  (bind _capsule (Variables|Collision|GetCapsule))
  (bind _returnvalue (Transformation|GetWorldLocation _capsule))
  (bind _newtrack_1 (Timeline|Timeline Play)
    (:Update
      (Transformation|SetWorldLocation _capsule (Math|Vector|MakeVector (.x _returnvalue) (.y _returnvalue) (+ (.z _returnvalue) _newtrack_1)) true false)
      (for _array_element (Collision|GetOverlappingActors (Variables|Collision|GetCapsule) 0 :!class /Script/Engine.PrimitiveComponent)
        (Development|PrintString (Utilities|GetDisplayName _array_element))))))

(event EventBeginPlay
  (bind _returnvalue (UserInterface|CreateWidget "/Game/Game/Widgets/MainUI/WBP_Diary.WBP_Diary_C"))
  (Variables|Default|SetDiaryUI _returnvalue)
  (bind _returnvalue_2 (UserInterface|CreateWidget "/Game/Game/Widgets/MainUI/WBP_UI.WBP_UI_C"))
  (Variables|Default|SetUI _returnvalue_2)
  (UserInterface|Viewport|AddtoViewport _returnvalue_2 0)
  (if (Variables|Default|GetIsAmuletOn)
    (Widget|SetVisibility (Variables|/Game/Game/Widgets/MainUI/WBP_UI.WBP_UI_C|GetProgressBar_2 (Variables|Default|GetUI)) "Visible")
    (Widget|SetVisibility (Variables|/Game/Game/Widgets/MainUI/WBP_UI.WBP_UI_C|Getmind_Image (Variables|Default|GetUI)) "Visible")
    (else
      (Widget|SetVisibility (Variables|/Game/Game/Widgets/MainUI/WBP_UI.WBP_UI_C|GetProgressBar_2 (Variables|Default|GetUI)) "Hidden")
      (Widget|SetVisibility (Variables|/Game/Game/Widgets/MainUI/WBP_UI.WBP_UI_C|Getmind_Image (Variables|Default|GetUI)) "Hidden"))))

(event Input|AxisEvents|InputAxisUp
  (params (AxisValue :type Float%20%28single-precision%29))
  (bind _arrow (Variables|Default|GetArrow))
  (bind _speed (Variables|Default|GetSpeed))
  (bind _capsule (Variables|Collision|GetCapsule))
  (bind _returnvalue (Transformation|GetWorldLocation _capsule))
  (bind _returnvalue_2 (Math|Vector|GetForwardVector _arrow))
  (bind _output_get (Variables|Default|SetAxisValueUp AxisValue))
  (Transformation|SetWorldLocation (Variables|Collision|GetCapsule) (Math|Vector|MakeVector (+ (* _output_get (* (.x _returnvalue_2) _speed)) (.x _returnvalue)) (+ (* _output_get (* (.y _returnvalue_2) _speed)) (.y _returnvalue)) (.z _returnvalue)) true false)
  (if (== (Variables|Default|GetAxisValueUp) 1.0)
    (Utilities|FlowControl|Delay 0.5 :!label _label)
    (Audio|SpawnSound2D "/Game/Game/Sounds/Walking.Walking" 0.1 1.0 0.0 0)
    (elif (== (Variables|Default|GetAxisValueUp) -1.0)
      (goto _label))))

(event Input|AxisEvents|InputAxisLeft
  (params (AxisValue :type Float%20%28single-precision%29))
  (bind _arrow (Variables|Default|GetArrow))
  (bind _speed (Variables|Default|GetSpeed))
  (bind _capsule (Variables|Collision|GetCapsule))
  (bind _returnvalue (Math|Vector|GetForwardVector _arrow))
  (bind _returnvalue_2 (Transformation|GetWorldLocation _capsule))
  (bind _output_get (Variables|Default|SetAxisValueLeft AxisValue))
  (Transformation|SetWorldLocation (Variables|Collision|GetCapsule) (Math|Vector|MakeVector (+ (* (* _output_get (* (.y _returnvalue) _speed)) -1.0) (.x _returnvalue_2)) (+ (* _output_get (* (.x _returnvalue) _speed)) (.y _returnvalue_2)) (.z _returnvalue_2)) true false)
  (if (== (Variables|Default|GetAxisValueLeft) 1.0)
    (if (== (Variables|Default|GetAxisValueUp) 0.0)
      (Utilities|FlowControl|Delay 0.5 :!label _label)
      (Audio|SpawnSound2D "/Game/Game/Sounds/Walking.Walking" 0.3 1.0 0.0 0))
    (elif (== (Variables|Default|GetAxisValueLeft) -1.0)
      (if (== (Variables|Default|GetAxisValueUp) 0.0)
        (goto _label)))))

(event Input|AxisEvents|InputAxisRotation
  (params (AxisValue :type Float%20%28single-precision%29))
  (Transformation|AddWorldRotation (Variables|Collision|GetCapsule) (Math|Rotator|MakeRotator 0.0 0.0 AxisValue) false false))

(event Input|KeyboardEvents|Escape
  (params (Key :type Key%20Structure :default "None"))
  (bind _returnvalue (Game|GetPlayerController 0))
  (:Pressed
    (bind _returnvalue_2 (UserInterface|CreateWidget "/Game/Game/Widgets/MainUI/WBP_EscMenu.WBP_EscMenu_C"))
    (UserInterface|Viewport|AddtoViewport _returnvalue_2 0)
    (Input|SetInputModeUIOnly _returnvalue _returnvalue_2 "DoNotLock" false)
    (Variables|/Script/Engine.PlayerController|SetbShowMouseCursor _returnvalue true)
    (Game|SetGamePaused true)))

(event Input|KeyboardEvents|E
  (params (Key :type Key%20Structure :default "None"))
  (:Pressed
    (for _array_element (Collision|GetOverlappingActors "/Script/Engine.Actor" :!class /Script/Engine.Actor)
      (if (Utilities|DoesObjectImplementInterface _array_element "/Game/Game/Door/BI_Interaction.BI_Interaction_C")
        (Variables|Default|SetInteractableActor _array_element)
        (Class|BIInteraction|Interaction(Message) (Variables|Default|GetInteractableActor))
        (Utilities|FlowControl|Delay 5.0)
        (Default|SayPhrase (Variables|/Game/Game/Widgets/MainUI/WBP_UI.WBP_UI_C|GetWBP_DynamicText_reusable (Variables|Default|GetUI)) " " 0.05)))))

(event Input|KeyboardEvents|Tab
  (params (Key :type Key%20Structure :default "None"))
  (bind _returnvalue (Game|GetPlayerController 0))
  (bind _diaryui (Variables|Default|GetDiaryUI))
  (:Pressed
    (UserInterface|Viewport|AddtoViewport _diaryui 0)
    (Input|SetInputModeUIOnly _returnvalue _diaryui "DoNotLock" false)
    (Variables|/Script/Engine.PlayerController|SetbShowMouseCursor _returnvalue true)
    (Game|SetGamePaused true)))

(event Input|KeyboardEvents|SpaceBar
  (params (Key :type Key%20Structure :default "None"))
  (bind _returnvalue (Transformation|GetActorLocation))
  (bind _tint_color (Variables|Default|GetTint%20Color))
  (:Pressed
    (if (Variables|Default|GetIsAmuletOn)
      (if (<= (Variables|Default|GetMind) 0.0)
        (bind _outactors (Actor|GetAllActorsOfClass "/Game/Game/Actors/BP_Hunter.BP_Hunter_C"))
        (if (== (Utilities|Array|Length _outactors) 0)
          (bind _returnvalue_2 (Game|SpawnActorfromClass "/Game/Game/Actors/BP_Hunter.BP_Hunter_C" (Math|Transform|MakeTransform (Math|Vector|MakeVector (+ (.x _returnvalue) 1e+02) (.y _returnvalue) (+ (.z _returnvalue) 6e+01)) "0, 0, 0" "1.000000,1.000000,1.000000") "Undefined" "MultiplyWithRoot" 0 0))
          (Development|PrintString (Utilities|String|ToString(Vector) (Transformation|GetSocketLocation (Variables|/Game/Game/Actors/BP_Hunter.BP_Hunter_C|GetDefaultSceneRoot _returnvalue_2) "None")))
          (Class|Image|SetBrushTintColor (Variables|/Game/Game/Widgets/MainUI/WBP_UI.WBP_UI_C|GetImage_0 (Variables|Default|GetUI)) (Variables|Default|GetTint%20Color)))
        (else
          (Variables|Default|SetMind (- (Variables|Default|GetMind) 1e+01))
          (Class|Image|SetBrushTintColor (Variables|/Game/Game/Widgets/MainUI/WBP_UI.WBP_UI_C|GetImage_0 (Variables|Default|GetUI)) (Utilities|Struct|MakeSlateColor (Utilities|Struct|MakeLinearColor (.r (.specifiedcolor _tint_color)) (.g (.specifiedcolor _tint_color)) (.b (.specifiedcolor _tint_color)) (- (.a (.specifiedcolor _tint_color)) (/ (Variables|Default|GetMind) 1e+02))) (.coloruserule _tint_color)))
          (Progress|SetPercent (Variables|/Game/Game/Widgets/MainUI/WBP_UI.WBP_UI_C|GetProgressBar_2 (Variables|Default|GetUI)) (/ (Variables|Default|GetMind) 1e+02))
          (CallFunction|MindChenger)
          (bind _outactors_2 (Collision|SphereOverlapActors (Transformation|GetWorldLocation (Variables|Collision|GetCapsule)) 3e+02 (Variables|Default|GetObject%20Types) 0 (Variables|Default|GetActors%20to%20Ignore)))
          (for _array_element _outactors_2
            (bind _asbp_active_things (Utilities|Casting|CastToBP_ActiveThings _array_element))
            (Utilities|Array|Add (Variables|Default|GetOut%20Actors) _asbp_active_things)
            (Rendering|Components|Light|SetLightColor (Variables|/Game/Game/Active/BP_ActiveThings.BP_ActiveThings_C|GetPointLight _asbp_active_things) "(R=0.522256,G=1.000000,B=0.203959,A=1.000000)" true)
            (Utilities|FlowControl|Delay 1.0)
            (for _array_element_2 (Variables|Default|GetOut%20Actors)
              (Rendering|Components|Light|SetLightColor (Variables|/Game/Game/Active/BP_ActiveThings.BP_ActiveThings_C|GetPointLight _array_element_2) "(R=0.000000,G=0.000000,B=0.000000,A=1.000000)" true))
            (Utilities|Array|Clear (Variables|Default|GetOut%20Actors)))))
      (else
        (Widget|SetVisibility (Variables|/Game/Game/Widgets/MainUI/WBP_UI.WBP_UI_C|GetProgressBar_2 (Variables|Default|GetUI)) "Hidden")))))

(event Input|KeyboardEvents|I
  (params (Key :type Key%20Structure :default "None"))
  (bind _returnvalue (Game|GetPlayerController 0))
  (:Pressed
    (bind _returnvalue_2 (UserInterface|CreateWidget "/Game/Game/Widgets/MainUI/WBP_EscMenu.WBP_EscMenu_C"))
    (UserInterface|Viewport|AddtoViewport _returnvalue_2 0)
    (Input|SetInputModeUIOnly _returnvalue _returnvalue_2 "DoNotLock" false)
    (Variables|/Script/Engine.PlayerController|SetbShowMouseCursor _returnvalue true)
    (Game|SetGamePaused true)))

(event Input|KeyboardEvents|C
  (params (Key :type Key%20Structure :default "None"))
  (bind _returnvalue (Transformation|GetActorLocation))
  (bind _tint_color (Variables|Default|GetTint%20Color))
  (:Pressed
    (if (Variables|Default|GetIsRingOn)
      (if (Variables|Default|GetInsideSW)
        (if (== (Variables|Default|GetMind) 0.0)
          (bind _outactors (Actor|GetAllActorsOfClass "/Game/Game/Actors/BP_Hunter.BP_Hunter_C"))
          (if (== (Utilities|Array|Length _outactors) 0)
            (Game|SpawnActorfromClass "/Game/Game/Actors/BP_Hunter.BP_Hunter_C" (Math|Transform|MakeTransform (Math|Vector|MakeVector (+ (.x _returnvalue) 1e+02) (.y _returnvalue) (+ (.z _returnvalue) 6e+01)) "0, 0, 0" "1.000000,1.000000,1.000000") "Undefined" "MultiplyWithRoot" 0 0)
            (Class|Image|SetBrushTintColor (Variables|/Game/Game/Widgets/MainUI/WBP_UI.WBP_UI_C|GetImage_0 (Variables|Default|GetUI)) (Variables|Default|GetTint%20Color)))
          (else
            (Development|PrintString "True")
            (Variables|Default|SetMind (- (Variables|Default|GetMind) 1e+01))
            (Class|Image|SetBrushTintColor (Variables|/Game/Game/Widgets/MainUI/WBP_UI.WBP_UI_C|GetImage_0 (Variables|Default|GetUI)) (Utilities|Struct|MakeSlateColor (Utilities|Struct|MakeLinearColor (.r (.specifiedcolor _tint_color)) (.g (.specifiedcolor _tint_color)) (.b (.specifiedcolor _tint_color)) (- (.a (.specifiedcolor _tint_color)) (/ (Variables|Default|GetMind) 1e+02))) (.coloruserule _tint_color)))
            (Progress|SetPercent (Variables|/Game/Game/Widgets/MainUI/WBP_UI.WBP_UI_C|GetProgressBar_2 (Variables|Default|GetUI)) (/ (Variables|Default|GetMind) 1e+02))
            (CallFunction|MindChenger)
            (bind _outactors_2 (Actor|GetAllActorswithTag "SecondWorld"))
            (Utilities|FlowControl|FlipFlop
              (:A
                (for _array_element _outactors_2
                  (Development|SetHiddeninGame (Variables|/Script/Engine.Actor|GetRootComponent _array_element) true true)
                  (Transformation|SetWorldLocation (Variables|/Script/Engine.Actor|GetRootComponent _array_element) (Math|Vector|MakeVector (.x (Transformation|GetWorldLocation (Variables|/Script/Engine.Actor|GetRootComponent _array_element))) (.y (Transformation|GetWorldLocation (Variables|/Script/Engine.Actor|GetRootComponent _array_element))) (- (.z (Transformation|GetWorldLocation (Variables|/Script/Engine.Actor|GetRootComponent _array_element))) 1e+03)) false true)
                  (bind _outactors_3 (Actor|GetAllActorswithTag "ThirdWorld"))
                  (for _array_element_2 _outactors_3
                    (bind _asbp_puzle (Utilities|Casting|CastToBP_Puzle _array_element_2))
                    (Default|ChangeHidden _asbp_puzle)
                    (Utilities|FlowControl|FlipFlop
                      (:A
                        (Transformation|SetWorldLocation (Variables|/Script/Engine.Actor|GetRootComponent _asbp_puzle) (Math|Vector|MakeVector (.x (Transformation|GetWorldLocation (Variables|/Script/Engine.Actor|GetRootComponent _asbp_puzle))) (.y (Transformation|GetWorldLocation (Variables|/Script/Engine.Actor|GetRootComponent _asbp_puzle))) (+ (.z (Transformation|GetWorldLocation (Variables|/Script/Engine.Actor|GetRootComponent _asbp_puzle))) 1e+03)) false true))
                      (:B
                        (Transformation|SetWorldLocation (Variables|/Script/Engine.Actor|GetRootComponent _asbp_puzle) (Math|Vector|MakeVector (.x (Transformation|GetWorldLocation (Variables|/Script/Engine.Actor|GetRootComponent _asbp_puzle))) (.y (Transformation|GetWorldLocation (Variables|/Script/Engine.Actor|GetRootComponent _asbp_puzle))) (+ (.z (Transformation|GetWorldLocation (Variables|/Script/Engine.Actor|GetRootComponent _asbp_puzle))) -1e+03)) false true))))))
              (:B
                (for _array_element_3 _outactors_2
                  (Development|SetHiddeninGame (Variables|/Script/Engine.Actor|GetRootComponent _array_element_3) false true)
                  (Transformation|SetWorldLocation (Variables|/Script/Engine.Actor|GetRootComponent _array_element_3) (Math|Vector|MakeVector (.x (Transformation|GetWorldLocation (Variables|/Script/Engine.Actor|GetRootComponent _array_element_3))) (.y (Transformation|GetWorldLocation (Variables|/Script/Engine.Actor|GetRootComponent _array_element_3))) (+ (.z (Transformation|GetWorldLocation (Variables|/Script/Engine.Actor|GetRootComponent _array_element_3))) 1e+03)) false true)
                  (bind _outactors_4 (Actor|GetAllActorswithTag "ThirdWorld"))
                  (for _array_element_4 _outactors_4
                    (bind _asbp_puzle_2 (Utilities|Casting|CastToBP_Puzle _array_element_4))
                    (Default|ChangeHidden _asbp_puzle_2)
                    (Utilities|FlowControl|FlipFlop
                      (:A
                        (Transformation|SetWorldLocation (Variables|/Script/Engine.Actor|GetRootComponent _asbp_puzle_2) (Math|Vector|MakeVector (.x (Transformation|GetWorldLocation (Variables|/Script/Engine.Actor|GetRootComponent _asbp_puzle_2))) (.y (Transformation|GetWorldLocation (Variables|/Script/Engine.Actor|GetRootComponent _asbp_puzle_2))) (+ (.z (Transformation|GetWorldLocation (Variables|/Script/Engine.Actor|GetRootComponent _asbp_puzle_2))) 1e+03)) false true))
                      (:B
                        (Transformation|SetWorldLocation (Variables|/Script/Engine.Actor|GetRootComponent _asbp_puzle_2) (Math|Vector|MakeVector (.x (Transformation|GetWorldLocation (Variables|/Script/Engine.Actor|GetRootComponent _asbp_puzle_2))) (.y (Transformation|GetWorldLocation (Variables|/Script/Engine.Actor|GetRootComponent _asbp_puzle_2))) (+ (.z (Transformation|GetWorldLocation (Variables|/Script/Engine.Actor|GetRootComponent _asbp_puzle_2))) -1e+03)) false true)))))))))))))

(fn ConstructionScript)

(fn MindChenger
  (bind _mind (Variables|Default|GetMind))
  (bind _ui (Variables|Default|GetUI))
  (bind _returnvalue (/ _mind 1e+02))
  (bind _mind_image (Variables|/Game/Game/Widgets/MainUI/WBP_UI.WBP_UI_C|Getmind_Image _ui))
  (if (== _returnvalue 0.6)
    (Appearance|SetBrushfromTexture _mind_image "/Game/Game/Widgets/MainUI/mind_Icon_60.mind_Icon_60" false)
    (elif (== _returnvalue 0.4)
      (Appearance|SetBrushfromTexture _mind_image "/Game/Game/Widgets/MainUI/mind_Icon_40.mind_Icon_40" false)
      (elif (== _returnvalue 0.2)
        (Appearance|SetBrushfromTexture _mind_image "/Game/Game/Widgets/MainUI/mind_Icon_20.mind_Icon_20" false)
        (elif (== _returnvalue 0.0)
          (Appearance|SetBrushfromTexture _mind_image "/Game/Game/Widgets/MainUI/mind_Icon_00.mind_Icon_00" false))))))

(fn Interaction
  (return true))