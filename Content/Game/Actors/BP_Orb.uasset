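; BP_Orb is a pickup that restores the player's Mind and works only while the player's amulet is on.
; On BeginPlay it hides itself if the first BP_Player found has the amulet off.
; A hit by an amulet-wearing player plays a sound and destroys the orb, adding Mind unless already at 100.
; A gain also adjusts a UI image's tint alpha and refreshes the Mind bar and text.
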(event EventBeginPlay
  (bind _outactors (Actor|GetAllActorsOfClass "/Game/Game/Actors/BP_Player.BP_Player_C"))
  (if (not (Variables|/Game/Game/Actors/BP_Player.BP_Player_C|GetIsAmuletOn (Utilities|Array|Get(acopy) _outactors)))
    (Development|SetHiddeninGame (Variables|Default|GetDefaultSceneRoot) true true)))

(event EventTick
  (params (DeltaSeconds :type Float%20%28single-precision%29)))

(event Collision|EventHit
  (params (MyComp :type Primitive%20Component%20Object%20Reference) (Other :type Actor%20Object%20Reference) (OtherComp :type Primitive%20Component%20Object%20Reference) (bSelfMoved :type Boolean) (HitLocation :type Vector :default "0, 0, 0") (HitNormal :type Vector :default "0, 0, 0") (NormalImpulse :type Vector :default "0, 0, 0") (Hit :type Hit%20Result%20Structure%20%28by%20ref%29))
  (bind _asbp_player (Utilities|Casting|CastToBP_Player Other))
  (if (Variables|/Game/Game/Actors/BP_Player.BP_Player_C|GetIsAmuletOn _asbp_player)
    (if (== (Variables|/Game/Game/Actors/BP_Player.BP_Player_C|GetMind _asbp_player) 1e+02)
      (Audio|SpawnSound2D "/Game/Game/Sounds/Orb.Orb" 0.3 1.0 0.0 0)
      (Actor|DestroyActor)
      (else
        (Variables|/Game/Game/Actors/BP_Player.BP_Player_C|SetMind _asbp_player (+ (Variables|/Game/Game/Actors/BP_Player.BP_Player_C|GetMind _asbp_player) 1e+01))
        (Class|Image|SetBrushTintColor (Variables|/Game/Game/Widgets/MainUI/WBP_UI.WBP_UI_C|GetImage_0 (Variables|/Game/Game/Actors/BP_Player.BP_Player_C|GetUI _asbp_player)) (Utilities|Struct|MakeSlateColor (Utilities|Struct|MakeLinearColor (.r (.specifiedcolor (Variables|/Game/Game/Actors/BP_Player.BP_Player_C|GetTint%20Color _asbp_player))) (.g (.specifiedcolor (Variables|/Game/Game/Actors/BP_Player.BP_Player_C|GetTint%20Color _asbp_player))) (.b (.specifiedcolor (Variables|/Game/Game/Actors/BP_Player.BP_Player_C|GetTint%20Color _asbp_player))) (- (.a (.specifiedcolor (Variables|/Game/Game/Actors/BP_Player.BP_Player_C|GetTint%20Color _asbp_player))) (/ (Variables|/Game/Game/Actors/BP_Player.BP_Player_C|GetMind _asbp_player) 1e+02))) (.coloruserule (Variables|/Game/Game/Actors/BP_Player.BP_Player_C|GetTint%20Color _asbp_player))))
        (Audio|SpawnSound2D "/Game/Game/Sounds/Orb.Orb" 0.3 1.0 0.0 0)
        (Actor|DestroyActor)
        (bind _asbp_player_2 (Utilities|Casting|CastToBP_Player (Game|Player|GetPlayerPawn 0)))
        (Progress|SetPercent (Variables|/Game/Game/Widgets/MainUI/WBP_UI.WBP_UI_C|GetProgressBar_2 (Variables|/Game/Game/Actors/BP_Player.BP_Player_C|GetUI _asbp_player_2)) (/ (Variables|/Game/Game/Actors/BP_Player.BP_Player_C|GetMind _asbp_player_2) 1e+02))
        (Rendering|Components|TextRender|SetText (Variables|/Game/Game/Widgets/MainUI/WBP_UI.WBP_UI_C|GetMindUI (Variables|/Game/Game/Actors/BP_Player.BP_Player_C|GetUI _asbp_player_2)) (Utilities|Text|ToText(String) (Utilities|String|Append "Mind: " (Utilities|String|ToString(Float) (Variables|/Game/Game/Actors/BP_Player.BP_Player_C|GetMind _asbp_player_2)))))))))

(fn ConstructionScript
  (Rendering|Material|SetMaterial (Variables|Default|GetSphere) 0 "/Game/Game/Actors/M_Orb.M_Orb"))