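; BP_Puzle is a rotation puzzle with two cone meshes that opens a linked BP_DoorForC.
; Overlapping players see an interaction prompt.
; Interaction turns the cone whose box holds the player by 90° yaw, then opens the door if both match their target yaws, with debug prints.
; BeginPlay drops the root 1000 units, and ChangeHidden alternates actor visibility through a FlipFlop.
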(event Custom|ChangeHidden
  (Utilities|FlowControl|FlipFlop
    (:A
      (Rendering|SetActorHiddenInGame false))
    (:B
      (Rendering|SetActorHiddenInGame true))))

(event Collision|EventActorBeginOverlap
  (params (OtherActor :type Actor%20Object%20Reference))
  (bind _asbp_player (Utilities|Casting|CastToBP_Player OtherActor))
  (Widget|SetVisibility (Variables|/Game/Game/Widgets/MainUI/WBP_UI.WBP_UI_C|GetInteractionText (Variables|/Game/Game/Actors/BP_Player.BP_Player_C|GetUI _asbp_player)) "Visible"))

(event Collision|EventActorEndOverlap
  (params (OtherActor :type Actor%20Object%20Reference))
  (bind _asbp_player (Utilities|Casting|CastToBP_Player OtherActor))
  (Widget|SetVisibility (Variables|/Game/Game/Widgets/MainUI/WBP_UI.WBP_UI_C|GetInteractionText (Variables|/Game/Game/Actors/BP_Player.BP_Player_C|GetUI _asbp_player)) "Hidden"))

(event EventBeginPlay
  (bind _defaultsceneroot (Variables|Default|GetDefaultSceneRoot))
  (bind _returnvalue (Transformation|GetWorldLocation _defaultsceneroot))
  (Transformation|SetWorldLocation _defaultsceneroot (Math|Vector|MakeVector (.x _returnvalue) (.y _returnvalue) (+ (.z _returnvalue) -1e+03)) false true))

(fn ConstructionScript
  (Components|StaticMesh|SetStaticMesh (Variables|Default|GetStaticMesh) "/Engine/BasicShapes/Cone.Cone")
  (Components|StaticMesh|SetStaticMesh (Variables|Default|GetStaticMesh1) "/Engine/BasicShapes/Cone.Cone"))

(fn NewFunction)

(fn Interaction
  (bind _staticmesh1 (Variables|Default|GetStaticMesh1))
  (bind _staticmesh (Variables|Default|GetStaticMesh))
  (bind _staticmesh_2 (Variables|Default|GetStaticMesh))
  (bind _staticmesh1_2 (Variables|Default|GetStaticMesh1))
  (bind _relativerotation (Variables|/Script/Engine.SceneComponent|GetRelativeRotation _staticmesh1))
  (bind _relativerotation_2 (Variables|/Script/Engine.SceneComponent|GetRelativeRotation _staticmesh))
  (bind _relativerotation_3 (Variables|/Script/Engine.SceneComponent|GetRelativeRotation _staticmesh1_2))
  (bind _relativerotation_4 (Variables|/Script/Engine.SceneComponent|GetRelativeRotation _staticmesh_2))
  (Utilities|Casting|CastToBP_Player (Utilities|Array|Get(acopy) (Collision|GetOverlappingActors (Variables|Default|GetBox) "/Game/Game/Actors/BP_Player.BP_Player_C" :!class /Script/Engine.PrimitiveComponent))
    (:then
      (Transformation|SetRelativeRotation _staticmesh (Math|Rotator|MakeRotator (.roll _relativerotation_2) (.pitch _relativerotation_2) (+ (.yaw _relativerotation_2) 9e+01)) false false))
    (:CastFailed
      (Utilities|Casting|CastToBP_Player (Utilities|Array|Get(acopy) (Collision|GetOverlappingActors (Variables|Default|GetBox1) "/Game/Game/Actors/BP_Player.BP_Player_C" :!class /Script/Engine.PrimitiveComponent)))
      (Transformation|SetRelativeRotation _staticmesh1 (Math|Rotator|MakeRotator (.roll _relativerotation) (.pitch _relativerotation) (+ (.yaw _relativerotation) 9e+01)) false false)))
  (if (Utilities|Operators|EqualEqual (Math|Rotator|MakeRotator (.roll _relativerotation_4) (.pitch _relativerotation_4) (.yaw _relativerotation_4)) (Math|Rotator|MakeRotator (.roll _relativerotation_4) (.pitch _relativerotation_4) 9e+01) 0.0)
    (Development|PrintString "Yes")
    (if (Utilities|Operators|EqualEqual (Math|Rotator|MakeRotator (.roll _relativerotation_3) (.pitch _relativerotation_3) (.yaw _relativerotation_3)) (Math|Rotator|MakeRotator (.roll _relativerotation_3) (.pitch _relativerotation_3) 1.8e+02) 0.0)
      (bind _asbp_door_for_c (Utilities|Casting|CastToBP_DoorForC (Variables|Default|GetDoor)))
      (Default|Open _asbp_door_for_c)
      (else
        (Development|PrintString "no")))
    (else
      (Development|PrintString "no")))
  (return false))