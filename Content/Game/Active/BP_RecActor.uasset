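; BP_RecActor is an actor whose Cube mesh can be rotated by dragging the mouse.
; Click start stores the mouse position and enables rotation, and click end disables it.
; While enabled, each mouse move adds world pitch and yaw scaled from the offset to the starting position, so rotation accumulates with every move event.
; The construction script sets the mesh and material from ActiveThing, with Book as the only case shown.
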(event Custom|Mouse%20Move
  (params (Mouse%20Move :type Vector%202D%20Structure))
  (bind _start_location (Variables|Default|GetStart%20location))
  (bind _returnvalue (- Mouse%20Move _start_location))
  (bind _returnvalue_2 (/ _returnvalue "(X=100.000000,Y=100.000000)"))
  (bind (_x _y) (Math|Vector2D|BreakVector2D _returnvalue_2))
  (if (Variables|Default|GetCan%20rotation)
    (Transformation|AddWorldRotation (Variables|Default|GetCube) (Math|Rotator|MakeRotator 0.0 _y (* _x -1.0)) false false)))

(event Custom|Click%20end
  (Variables|Default|SetCan%20rotation false))

(event Custom|Click%20start
  (params (Mouse%20location :type Vector%202D%20Structure))
  (Variables|Default|SetStart%20location Mouse%20location)
  (Variables|Default|SetCan%20rotation true))

(fn ConstructionScript
  (bind _cube (Variables|Default|GetCube))
  (switch Utilities|FlowControl|Switch|SwitchonThingENum (Variables|Default|GetActiveThing)
    (:NewEnumerator0
      (Components|StaticMesh|SetStaticMesh _cube "/Game/Game/Models/Models_filling/small_things/Book.Book")
      (Rendering|Material|SetMaterial _cube 0 "/Game/Game/Models/Models_filling/small_things/Material_small_things/Book_2.Book_2"))))