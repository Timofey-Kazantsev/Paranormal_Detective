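; BP_ActiveThings is an interactable world object that switches on its Thing variable and speaks a line through the player's UI.
; On overlap with a BP_Player, it caches that player's UI widget.
; Interaction enables talking on the dynamic text widget, types out a hardcoded placeholder-like phrase letter by letter, prints the result and returns false.
; The construction script's switch on Thing drives no logic.
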(event EventBeginPlay)

(event Collision|EventActorBeginOverlap
  (params (OtherActor :type Actor%20Object%20Reference))
  (bind _asbp_player (Utilities|Casting|CastToBP_Player OtherActor))
  (Variables|Default|SetUIWidget (Variables|/Game/Game/Actors/BP_Player.BP_Player_C|GetUI _asbp_player)))

(event EventTick
  (params (DeltaSeconds :type Float%20%28single-precision%29)))

(fn ConstructionScript
  (switch Utilities|FlowControl|Switch|SwitchonThingENum (Variables|Default|GetThing)))

(fn Interaction
  (bind _uiwidget (Variables|Default|GetUIWidget))
  (bind _wbp_dynamictext_reusable (Variables|/Game/Game/Widgets/MainUI/WBP_UI.WBP_UI_C|GetWBP_DynamicText_reusable _uiwidget))
  (switch Utilities|FlowControl|Switch|SwitchonThingENum (Variables|Default|GetThing)
    (:NewEnumerator0
      (Variables|/Game/Game/Widgets/MainUI/WBP_DynamicText_reusable.WBP_DynamicText_reusable_C|SetbIsTalkingAllowed _wbp_dynamictext_reusable true)
      (bind _phraseduration (Default|SayPhrase _wbp_dynamictext_reusable "I am babushka hahui 
How are you ebani v rot?" 0.05))
      (Development|PrintString (Utilities|String|ToString(Float) _phraseduration))
      (return false))))