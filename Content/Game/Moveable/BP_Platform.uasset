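; BP_Platform is a puzzle platform that reports to a BP_PlatformController when a BP_Moveable rests on it.
; On begin overlap it adds itself to the controller's AlreadyOverlapedPassPlat collection and triggers CheckPassword.
; On end overlap it removes itself from that collection without rechecking the password.
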(event Collision|EventActorBeginOverlap
  (params (OtherActor :type Actor%20Object%20Reference))
  (Utilities|Casting|CastToBP_Moveable OtherActor)
  (bind _asbp_platform_controller (Utilities|Casting|CastToBP_PlatformController (Variables|Default|GetController)))
  (Utilities|Array|Add (Variables|/Game/Game/Moveable/BP_PlatformController.BP_PlatformController_C|GetAlreadyOverlapedPassPlat _asbp_platform_controller) self)
  (Default|CheckPassword (Variables|Default|GetController)))

(event Collision|EventActorEndOverlap
  (params (OtherActor :type Actor%20Object%20Reference))
  (Utilities|Casting|CastToBP_Moveable OtherActor)
  (bind _asbp_platform_controller (Utilities|Casting|CastToBP_PlatformController (Variables|Default|GetController)))
  (Utilities|Array|RemoveItem (Variables|/Game/Game/Moveable/BP_PlatformController.BP_PlatformController_C|GetAlreadyOverlapedPassPlat _asbp_platform_controller) self))

(fn ConstructionScript)