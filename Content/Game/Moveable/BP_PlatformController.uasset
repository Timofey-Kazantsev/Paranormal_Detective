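; BP_PlatformController runs a password puzzle in which overlapped platforms must match an expected order to open a door.
; CheckPassword compares AlreadyOverlapedPassPlat to PasswordPlatforms by index, adding matches to a running ActivatedPlatforms count that is never reset here.
; It subtracts an escalating Minus, reset on mismatches, when the count is neither zero nor one, then calls OpenDoor if it equals LenPassword.
; An older debug-printing version of the check remains disconnected.
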(event Custom|CheckPassword
  (for (_array_element _array_index) (Variables|Default|GetAlreadyOverlapedPassPlat)
    (if (== (Utilities|Array|Get(acopy) (Variables|Default|GetPasswordPlatforms) _array_index) _array_element)
      (Variables|Default|SetActivatedPlatforms (+ (Variables|Default|GetActivatedPlatforms) 1))
      (else
        (Variables|Default|SetMinus 1))))
  (if (== (Variables|Default|GetActivatedPlatforms) 1)
    _
    (elif (== (Variables|Default|GetActivatedPlatforms) 0)
      _
      (else
        (Variables|Default|SetActivatedPlatforms (- (Variables|Default|GetActivatedPlatforms) (Variables|Default|GetMinus)))
        (Variables|Default|SetMinus (+ (Variables|Default|GetMinus) 1)))))
  (if (== (Variables|Default|GetActivatedPlatforms) (Variables|Default|GetLenPassword))
    (Default|OpenDoor (Variables|Default|GetDoor))))

(fn ConstructionScript)