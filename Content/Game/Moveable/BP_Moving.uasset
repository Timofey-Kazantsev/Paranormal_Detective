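; BP_Moving is the in-motion form of a movable object, following the player until dropped.
; Each Tick sweeps the Cube toward the player's XY, keeping its height and yawing to face them.
; Exceeding 200 units separation on X or Y, or interacting while IsMoveingItem is set, replaces it with a spawned BP_Moveable.
; Player overlap toggles the interaction prompt; Dropping duplicates the distance check but is uncalled here.
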(event Collision|EventActorBeginOverlap
  (params (OtherActor :type Actor%20Object%20Reference))
  (bind _asbp_player (Utilities|Casting|CastToBP_Player OtherActor))
  (Widget|SetVisibility (Variables|/Game/Game/Widgets/MainUI/WBP_UI.WBP_UI_C|GetInteractionText (Variables|/Game/Game/Actors/BP_Player.BP_Player_C|GetUI _asbp_player)) "Visible"))

(event Collision|EventActorEndOverlap
  (params (OtherActor :type Actor%20Object%20Reference))
  (bind _asbp_player (Utilities|Casting|CastToBP_Player OtherActor))
  (Widget|SetVisibility (Variables|/Game/Game/Widgets/MainUI/WBP_UI.WBP_UI_C|GetInteractionText (Variables|/Game/Game/Actors/BP_Player.BP_Player_C|GetUI _asbp_player)) "Hidden"))

(event EventTick
  (params (DeltaSeconds :type Float%20%28single-precision%29))
  (bind _cube (Variables|Default|GetCube))
  (bind _cube_2 (Variables|Default|GetCube))
  (bind _returnvalue (Transformation|GetWorldLocation _cube_2))
  (bind _outactors (Actor|GetAllActorsOfClass "/Game/Game/Actors/BP_Player.BP_Player_C"))
  (bind _output_get (Variables|Default|SetPlayer (Utilities|Array|Get(acopy) _outactors)))
  (bind _asbp_player (Utilities|Casting|CastToBP_Player _output_get))
  (Variables|Default|SetZrotator (.yaw (.rotation (Class|KismetAnimationLibrary|Lookat (Transformation|GetWorldTransform (Variables|Default|GetCube)) (Transformation|GetWorldLocation (Variables|/Game/Game/Actors/BP_Player.BP_Player_C|GetCapsule _asbp_player)) "1.000000,0.000000,0.000000" false "0, 0, 0" 0.0))))
  (if (>= (- (.x _returnvalue) (.x (Transformation|GetWorldLocation (Variables|/Game/Game/Actors/BP_Player.BP_Player_C|GetCapsule (Variables|Default|GetPlayer))))) 2e+02)
    (CallFunction|DropObject)
    (elif (<= (- (.x _returnvalue) (.x (Transformation|GetWorldLocation (Variables|/Game/Game/Actors/BP_Player.BP_Player_C|GetCapsule (Variables|Default|GetPlayer))))) -2e+02)
      (CallFunction|DropObject)
      (elif (>= (- (.y _returnvalue) (.y (Transformation|GetWorldLocation (Variables|/Game/Game/Actors/BP_Player.BP_Player_C|GetCapsule (Variables|Default|GetPlayer))))) 2e+02)
        (CallFunction|DropObject)
        (elif (<= (- (.y _returnvalue) (.y (Transformation|GetWorldLocation (Variables|/Game/Game/Actors/BP_Player.BP_Player_C|GetCapsule (Variables|Default|GetPlayer))))) -2e+02)
          (CallFunction|DropObject)
          (else
            (Transformation|SetWorldLocationAndRotation _cube (Math|Vector|MakeVector (.x (.location (Transformation|GetWorldTransform (Variables|/Game/Game/Actors/BP_Player.BP_Player_C|GetCapsule _asbp_player)))) (.y (.location (Transformation|GetWorldTransform (Variables|/Game/Game/Actors/BP_Player.BP_Player_C|GetCapsule _asbp_player)))) (.z (Transformation|GetWorldLocation _cube))) (Math|Rotator|MakeRotator 0.0 0.0 (Variables|Default|GetZrotator)) true false)))))))

(fn ConstructionScript)

(fn DropObject
  (bind _cube (Variables|Default|GetCube))
  (bind _returnvalue (Transformation|GetWorldTransform _cube))
  (Variables|/Game/Game/Actors/BP_Player.BP_Player_C|SetIsMoveingItem (Variables|Default|GetPlayer) false)
  (Game|SpawnActorfromClass "/Game/Game/Moveable/BP_Moveable.BP_Moveable_C" (Math|Transform|MakeTransform (.location _returnvalue) (.rotation _returnvalue) "1.000000,1.000000,1.000000") "Undefined" "MultiplyWithRoot" 0 0)
  (Actor|DestroyActor))

(fn Dropping
  (bind _cube (Variables|Default|GetCube))
  (bind _player (Variables|Default|GetPlayer))
  (bind _returnvalue (Transformation|GetWorldLocation _cube))
  (bind _capsule (Variables|/Game/Game/Actors/BP_Player.BP_Player_C|GetCapsule _player))
  (bind _returnvalue_2 (Transformation|GetWorldLocation _capsule))
  (bind _returnvalue_3 (- (.x _returnvalue) (.x _returnvalue_2)))
  (bind _returnvalue_4 (- (.y _returnvalue) (.y _returnvalue_2)))
  (if (>= _returnvalue_3 2e+02)
    (CallFunction|DropObject)
    (elif (<= _returnvalue_3 -2e+02)
      (CallFunction|DropObject)
      (elif (>= _returnvalue_4 2e+02)
        (CallFunction|DropObject)
        (elif (<= _returnvalue_4 -2e+02)
          (CallFunction|DropObject))))))

(fn Interaction
  (bind _cube (Variables|Default|GetCube))
  (bind _returnvalue (Transformation|GetWorldTransform _cube))
  (bind _asbp_player (Utilities|Casting|CastToBP_Player (Utilities|Array|Get(acopy) (Collision|GetOverlappingActors (Variables|Default|GetBox) "/Game/Game/Actors/BP_Player.BP_Player_C" :!class /Script/Engine.PrimitiveComponent))))
  (bind _output_get (Variables|Default|SetPlayer _asbp_player))
  (if (== (Variables|/Game/Game/Actors/BP_Player.BP_Player_C|GetIsMoveingItem _output_get) false)
    (Variables|/Game/Game/Actors/BP_Player.BP_Player_C|SetIsMoveingItem (Variables|Default|GetPlayer) true)
    (else
      (Variables|/Game/Game/Actors/BP_Player.BP_Player_C|SetIsMoveingItem (Variables|Default|GetPlayer) false)
      (Game|SpawnActorfromClass "/Game/Game/Moveable/BP_Moveable.BP_Moveable_C" (Math|Transform|MakeTransform (.location _returnvalue) (.rotation _returnvalue) "0.700000,0.700000,0.700000") "Undefined" "MultiplyWithRoot" 0 0)
      (Actor|DestroyActor)))
  (return false))