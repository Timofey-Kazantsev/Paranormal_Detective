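; BP_Moveable is a movable cube that the player can pick up through an interaction.
; Overlap events show and hide the interaction text on the BP_Player UI.
; Interaction finds the first player overlapping its Box and, if not already moving an item, flags them as moving, spawns BP_Moving at the cube's transform and destroys itself.
; If the player is already moving an item, it only clears that flag.
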(event Collision|EventActorBeginOverlap
  (params (OtherActor :type Actor%20Object%20Reference))
  (bind _asbp_player (Utilities|Casting|CastToBP_Player OtherActor))
  (Widget|SetVisibility (Variables|/Game/Game/Widgets/MainUI/WBP_UI.WBP_UI_C|GetInteractionText (Variables|/Game/Game/Actors/BP_Player.BP_Player_C|GetUI _asbp_player)) "Visible"))

(event Collision|EventActorEndOverlap
  (params (OtherActor :type Actor%20Object%20Reference))
  (bind _asbp_player (Utilities|Casting|CastToBP_Player OtherActor))
  (Widget|SetVisibility (Variables|/Game/Game/Widgets/MainUI/WBP_UI.WBP_UI_C|GetInteractionText (Variables|/Game/Game/Actors/BP_Player.BP_Player_C|GetUI _asbp_player)) "Hidden"))

(fn ConstructionScript
  (Transformation|SetWorldScale3D (Variables|Default|GetCube) "0.700000,0.700000,0.700000"))

(fn Interaction
  (bind _cube (Variables|Default|GetCube))
  (bind _returnvalue (Transformation|GetWorldTransform _cube))
  (bind _asbp_player (Utilities|Casting|CastToBP_Player (Utilities|Array|Get(acopy) (Collision|GetOverlappingActors (Variables|Default|GetBox) "/Game/Game/Actors/BP_Player.BP_Player_C" :!class /Script/Engine.PrimitiveComponent))))
  (bind _output_get (Variables|Default|SetPlayer _asbp_player))
  (if (== (Variables|/Game/Game/Actors/BP_Player.BP_Player_C|GetIsMoveingItem _output_get) false)
    (Variables|/Game/Game/Actors/BP_Player.BP_Player_C|SetIsMoveingItem (Variables|Default|GetPlayer) true)
    (Game|SpawnActorfromClass "/Game/Game/Moveable/BP_Moving.BP_Moving_C" (Math|Transform|MakeTransform (.location _returnvalue) (.rotation _returnvalue) "0.700000,0.700000,0.700000") "Undefined" "MultiplyWithRoot" 0 0)
    (Actor|DestroyActor)
    (else
      (Variables|/Game/Game/Actors/BP_Player.BP_Player_C|SetIsMoveingItem (Variables|Default|GetPlayer) false)))
  (return false))